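; Actor that shows directional cover icons at a grid position, marking half or full cover to the north, east, south and west.
; BeginPlay hides all eight icon components.
; DisplayCoverIcons stores the given cover data, moves the actor to the supplied grid position, and sets each icon's visibility from the matching flag in that data.
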(event `self.ReceiveBeginPlay`
  (`SceneComponent.SetVisibility` (`self.NorthHalfCover`) false false)
  (`SceneComponent.SetVisibility` (`self.EastHalfCover`) false false)
  (`SceneComponent.SetVisibility` (`self.SouthHalfCover`) false false)
  (`SceneComponent.SetVisibility` (`self.WestHalfCover`) false false)
  (`SceneComponent.SetVisibility` (`self.NorthFullCover`) false false)
  (`SceneComponent.SetVisibility` (`self.WestFullCover`) false false)
  (`SceneComponent.SetVisibility` (`self.SouthFullCover`) false false)
  (`SceneComponent.SetVisibility` (`self.EastFullCover`) false false))

(event `self.DisplayCoverIcons`
  (params (Cover :type "Cover Structure") (GridPosition :type "Vector Structure"))
  (bind (_cover_northhalfcover _cover_easthalfcover _cover_southhalfcover _cover_westhalfcover _cover_northfullcover _cover_eastfullcover _cover_southfullcover _cover_westfullcover) (break `Cover` (`self.Cover`)))
  (set `self.Cover` Cover)
  (`self.K2_SetActorLocation` GridPosition)
  (`SceneComponent.SetVisibility` (`self.NorthHalfCover`) _cover_northhalfcover false)
  (`SceneComponent.SetVisibility` (`self.EastHalfCover`) _cover_easthalfcover false)
  (`SceneComponent.SetVisibility` (`self.SouthHalfCover`) _cover_southhalfcover false)
  (`SceneComponent.SetVisibility` (`self.WestHalfCover`) _cover_westhalfcover false)
  (`SceneComponent.SetVisibility` (`self.NorthFullCover`) _cover_northfullcover false)
  (`SceneComponent.SetVisibility` (`self.EastFullCover`) _cover_eastfullcover false)
  (`SceneComponent.SetVisibility` (`self.SouthFullCover`) _cover_southfullcover false)
  (`SceneComponent.SetVisibility` (`self.WestFullCover`) _cover_westfullcover false))

(fn `UserConstructionScript`)