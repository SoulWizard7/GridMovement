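; BP_CameraController is a free-moving camera controller that pans, turns and zooms from player axis inputs.
; Forward and right axes offset the actor in local space by CameraMoveSpeed, and the turn axis adds world yaw directly.
; Zoom moves the actor along its local Z by ZoomAmount rather than changing FOV or arm length, with no clamping.
; BeginPlay stores the starting height in ZoomValue, which the graph never reads.
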(event `self.ReceiveBeginPlay`
  (bind (_returnvalue_x _returnvalue_y _returnvalue_z) (`KismetMathLibrary.BreakVector` (`self.K2_GetActorLocation`)))
  ;[1 1 1] Camera Movement and zoom
  (set `self.ZoomValue` _returnvalue_z))

(event `InputAxis|MoveCameraForward`
  (params (AxisValue :type "Float (single-precision)"))
  ;[1 1 1] Camera Movement and zoom
  (`self.K2_AddActorLocalOffset` (`KismetMathLibrary.MakeVector` (* AxisValue (`self.CameraMoveSpeed`)))))

(event `InputAxis|MoveCameraRight`
  (params (AxisValue :type "Float (single-precision)"))
  ;[1 1 1] Camera Movement and zoom
  (`self.K2_AddActorLocalOffset` (`KismetMathLibrary.MakeVector` 0.0 (* AxisValue (`self.CameraMoveSpeed`)))))

(event `InputAxis|TurnCamera`
  (params (AxisValue :type "Float (single-precision)"))
  ;[1 1 1] Camera Movement and zoom
  (`self.K2_AddActorWorldRotation` (`KismetMathLibrary.MakeRotator` 0.0 0.0 AxisValue)))

(event `InputAxis|ZoomAxis`
  (params (AxisValue :type "Float (single-precision)"))
  ;[1 1 1] Camera Movement and zoom
  (`self.K2_AddActorLocalOffset` (`KismetMathLibrary.MakeVector` 0.0 0.0 (* AxisValue (`self.ZoomAmount`)))))

(fn `UserConstructionScript`)