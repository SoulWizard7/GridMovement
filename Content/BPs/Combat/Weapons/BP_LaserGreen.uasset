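; BP_LaserGreen is a green laser projectile actor that self-destructs five seconds after spawning.
; Each tick it moves a fixed, frame-rate-dependent step along its cylinder's negative up vector without sweeping.
; With Reflect set, overlapping the ToAttack GMUnit randomly rolls the cylinder to deflect it, while other overlaps destroy it with a Niagara hit effect.
; Otherwise, only overlapping ToAttack triggers that effect and destruction; no damage is applied here.
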(event `self.ReceiveBeginPlay`
  (`KismetSystemLibrary.Delay` 5.0)
  (`self.K2_DestroyActor`))

(event `self.ReceiveTick`
  (params (DeltaSeconds :type "Float (single-precision)"))
  (`self.K2_AddActorWorldOffset` (* (`SceneComponent.GetUpVector` (`self.Cylinder`)) -40.0)))

(event `self.ReceiveActorBeginOverlap`
  (params (OtherActor :type "Actor Object Reference"))
  (if (`self.Reflect`)
    (bind _asgmunit (cast `GMUnit` OtherActor)
      (:`then`
        (if (== _asgmunit (`self.ToAttack`))
          (`SceneComponent.K2_AddLocalRotation` (`self.Cylinder`) (`KismetMathLibrary.MakeRotator` (`KismetMathLibrary.RandomFloatInRange` 90.0 270.0)) false false)
          (else
            (`self.HitEffectAndDestroy`))))
      (:`CastFailed`
        (`self.HitEffectAndDestroy` :!label _label)))
    (else
      (bind _asgmunit_2 (cast `GMUnit` OtherActor))
      (if (== _asgmunit_2 (`self.ToAttack`))
        (goto _label)))))

(fn `HitEffectAndDestroy`
  (`NiagaraFunctionLibrary.SpawnSystemAtLocation` "/Game/BPs/Combat/Weapons/NS_LaserHit.NS_LaserHit" (+ (`self.K2_GetActorLocation`) (* (`self.GetActorForwardVector`) 20.0)))
  (`self.K2_DestroyActor`))

(fn `UserConstructionScript`)