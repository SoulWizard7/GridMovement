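; BP_CombatManager sequences the enemy turn in combat, handing control to one BP_Enemy at a time from EnemyUnits.
; Tick polls MoveToNextUnit to call EnemyTurn on the unit at CurrentEnemyIndex, or end the enemy turn past the list's end, and prints debug values.
; The index is never incremented here.
; The CombatEnemyTurn event is empty, and the logic that resets the index to start a turn is disconnected.
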(event `self.CombatEnemyTurn.CombatEnemyTurnEvent`)

(event `self.ReceiveTick`
  (params (DeltaSeconds :type "Float (single-precision)"))
  (`KismetSystemLibrary.PrintString` (`KismetStringLibrary.Concat_StrStr` "current Enemy index: " (`KismetStringLibrary.Conv_IntToString` (`self.CurrentEnemyIndex`))) true true (struct :`G` 0.66 :`B` 1.0 :`A` 1.0) 0.0)
  (`KismetSystemLibrary.PrintString` (`KismetStringLibrary.Concat_StrStr` "Enemy units list lenght: " (`KismetStringLibrary.Conv_IntToString` (`KismetArrayLibrary.Array_Length` (`self.EnemyUnits`)))) true true (struct :`G` 0.66 :`B` 1.0 :`A` 1.0) 0.0)
  (if (`self.MoveToNextUnit`)
    (set `self.MoveToNextUnit` false)
    (if (> (+ (`self.CurrentEnemyIndex`) 1) (`KismetArrayLibrary.Array_Length` (`self.EnemyUnits`)))
      (`self.CombatManagerEndEnemyTurn`)
      (set `self.IsEnemyTurn` true)
      (else
        (bind _asbp_enemy (cast `/Game/BPs/Units/BP_Enemy` (`|GetArrayItem` (`self.EnemyUnits`) (`self.CurrentEnemyIndex`))))
        (`/Game/BPs/Units/BP_Enemy.EnemyTurn` _asbp_enemy)))))

(fn `UserConstructionScript`)