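; BP_EnemyBaseAIController is the base AI controller for enemy units, preparing Blackboard references for their AI.
; After a short delay on BeginPlay, it caches the possessed BP_Enemy and the top-down player controller, then writes both to Blackboard object keys.
; MoveToPos is an empty event; the call that would forward movement to the player controller's MoveEnemyUnit is disconnected.
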(event `self.ReceiveTick`
  (params (DeltaSeconds :type "Float (single-precision)")))

(event `self.ReceiveBeginPlay`
  (`KismetSystemLibrary.Delay` 0.2)
  (bind _asbp_enemy (cast `/Game/BPs/Units/BP_Enemy` (`self.K2_GetPawn`)))
  (bind _output_get (set `self.Self_BP_Ememy` _asbp_enemy))
  (`BlackboardComponent.SetValueAsObject` (`self.Blackboard`) "SelfBP_Enemy" _output_get)
  (bind _asbp_top_down_player_controller (cast `/Game/TopDown/Blueprints/BP_TopDownPlayerController` (`GameplayStatics.GetPlayerController` 0)))
  (bind _output_get_2 (set `self.GMPlayerController` _asbp_top_down_player_controller))
  (`BlackboardComponent.SetValueAsObject` (`self.Blackboard`) "BP_PlayerController" _output_get_2))

(event `MoveToPos`
  (params (NewPosition :type "Vector Structure")))

(fn `UserConstructionScript`)