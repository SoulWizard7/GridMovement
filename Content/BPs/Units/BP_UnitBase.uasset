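; Base unit Blueprint that handles grid movement and laser attacks.
; MovetoLocation finds a path with GMNavigator, navigates it and shows it through GMPathVisualizer, which Tick clears when the spline has no points.
; Attack and RTAttack turn toward the target and spawn green or standard lasers, with misses randomly offset sideways and flagged Reflect.
; Only Attack signals that the unit's action is done, while RTAttack serves as the real-time variant.
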(event `self.ReceiveBeginPlay`
  (bind _asgrid_movement_player_controller (cast `GridMovementPlayerController` (`GameplayStatics.GetPlayerController` 0)))
  (set `self.PlayerController` _asgrid_movement_player_controller))

(event `self.ReceiveTick`
  (params (DeltaSeconds :type "Float (single-precision)"))
  (if (not (>= (`SplineComponent.GetNumberOfSplinePoints` (`GMNavigatorComponent.Spline` (`self.GMNavigator`))) 1))
    (`GMNavigatorComponent.Stop` (`self.GMNavigator`))
    (`GMPathVisualizerComponent.SetWaypoints` (`self.GMPathVisualizer`) (`self.EmptyArrayOfVectors`))))

(event `self.Attack`
  (params (toAttack :type "GMUnit Object Reference") (hit :type Boolean))
  (bind _returnvalue (`KismetMathLibrary.MakeRotFromX` (`KismetMathLibrary.Normal` (- (`self.K2_GetActorLocation` toAttack) (`self.K2_GetActorLocation`)))))
  (bind _returnvalue_2 (+ (* (`self.GetActorUpVector`) 20.0) (+ (`self.K2_GetActorLocation`) (* (`self.GetActorForwardVector`) 100.0))))
  ;[1 0.5318 0.9822] Action Attack
  (`KismetSystemLibrary.PrintString` "Event Attack" true true (struct :`G` 1.0 :`B` 0.02428 :`A` 1.0) 4.0)
  (if hit
    (`self.K2_SetActorRotation` _returnvalue)
    (`KismetSystemLibrary.Delay` 0.2)
    (bind _returnvalue_3 (`|SpawnActorFromClass` "/Game/BPs/Combat/Weapons/BP_LaserGreen.BP_LaserGreen_C" (`KismetMathLibrary.MakeTransform` _returnvalue_2 _returnvalue) "AlwaysSpawn" "OverrideRootScale" null null))
    (set `/Game/BPs/Combat/Weapons/BP_LaserGreen.ToAttack` toAttack _returnvalue_3)
    (else
      (`self.K2_SetActorRotation` _returnvalue)
      (`KismetSystemLibrary.Delay` 0.2)
      (bind _returnvalue_4 (`|SpawnActorFromClass` "/Game/BPs/Combat/Weapons/BP_LaserGreen.BP_LaserGreen_C" (`KismetMathLibrary.MakeTransform` _returnvalue_2 (`KismetMathLibrary.MakeRotFromX` (`KismetMathLibrary.Normal` (- (+ (`self.K2_GetActorLocation` toAttack) (* (`self.GetActorRightVector`) (`KismetMathLibrary.RandomFloatInRange` -100.0 100.0))) (`self.K2_GetActorLocation`))))) "AlwaysSpawn" "OverrideRootScale" null null))
      (set `/Game/BPs/Combat/Weapons/BP_LaserGreen.Reflect` true _returnvalue_4)
      (set `/Game/BPs/Combat/Weapons/BP_LaserGreen.ToAttack` toAttack _returnvalue_4)))
  (`KismetSystemLibrary.Delay` 1.0)
  (`self.UnitIsDoneWithAction`))

(event `self.RTAttack`
  (params (toAttack :type "GMUnit Object Reference") (hit :type Boolean))
  (bind _returnvalue (`KismetMathLibrary.MakeRotFromX` (`KismetMathLibrary.Normal` (- (`self.K2_GetActorLocation` toAttack) (`self.K2_GetActorLocation`)))))
  (bind _returnvalue_2 (+ (* (`self.GetActorUpVector`) 20.0) (+ (`self.K2_GetActorLocation`) (* (`self.GetActorForwardVector`) 100.0))))
  ;[1 0.2488 0.2289] RealTime Attack
  (if hit
    (`self.K2_SetActorRotation` _returnvalue)
    (`KismetSystemLibrary.Delay` 0.2)
    (bind _returnvalue_3 (`|SpawnActorFromClass` "/Game/BPs/Combat/Weapons/BP_Laser.BP_Laser_C" (`KismetMathLibrary.MakeTransform` _returnvalue_2 _returnvalue) "AlwaysSpawn" "OverrideRootScale" null null))
    (set `/Game/BPs/Combat/Weapons/BP_Laser.ToAttack` toAttack _returnvalue_3)
    (else
      (`self.K2_SetActorRotation` _returnvalue)
      (`KismetSystemLibrary.Delay` 0.2)
      (bind _returnvalue_4 (`|SpawnActorFromClass` "/Game/BPs/Combat/Weapons/BP_Laser.BP_Laser_C" (`KismetMathLibrary.MakeTransform` _returnvalue_2 (`KismetMathLibrary.MakeRotFromX` (`KismetMathLibrary.Normal` (- (+ (`self.K2_GetActorLocation` toAttack) (* (`self.GetActorRightVector`) (`KismetMathLibrary.RandomFloatInRange` -100.0 100.0))) (`self.K2_GetActorLocation`))))) "AlwaysSpawn" "OverrideRootScale" null null))
      (set `/Game/BPs/Combat/Weapons/BP_Laser.Reflect` true _returnvalue_4)
      (set `/Game/BPs/Combat/Weapons/BP_Laser.ToAttack` toAttack _returnvalue_4))))

(event `self.MoveToLocation`
  (params (NewLocation :type "Vector Structure"))
  (bind _gmnavigator (`self.GMNavigator`))
  ;[0.3702 1 0.4144] Movement Function
  (`KismetSystemLibrary.Delay` 0.5)
  (bind _returnvalue (`GMNavigatorComponent.FindPathToLocation` _gmnavigator NewLocation))
  (`GMNavigatorComponent.Navigate` _gmnavigator _returnvalue)
  (`GMPathVisualizerComponent.SetWaypoints` (`self.GMPathVisualizer`) _returnvalue)
  (`KismetSystemLibrary.PrintString` "end"))

(fn `UserConstructionScript`)