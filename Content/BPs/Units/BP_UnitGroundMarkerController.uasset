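; BP_UnitGroundMarkerController is a component that switches the ground marker decal under a unit to show its interaction state.
; On BeginPlay it casts its owner to BP_UnitBase and caches that unit's UnitGroundMarker, printing an error on screen if the cast fails.
; Four events swap the decal material between default, selected, hover-to-attack and hover-to-select looks.
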(event `self.ReceiveBeginPlay`
  (bind _asbp_unit_base (cast `/Game/BPs/Units/BP_UnitBase` (`self.GetOwner`))
    (:`then`
      (bind _output_get (set `self.Owner` _asbp_unit_base))
      (set `self.GroundMarker` (`GMUnit.UnitGroundMarker` _output_get)))
    (:`CastFailed`
      (`KismetSystemLibrary.PrintString` "Ground marker cast to unit failed" true true (struct :`R` 1.0 :`G` 0.034709 :`A` 1.0) 10.0))))

(event `self.SetDecalDefault`
  (`DecalComponent.SetDecalMaterial` (`self.GroundMarker`) (`self.Default`)))

(event `self.SetDecalSelected`
  (`DecalComponent.SetDecalMaterial` (`self.GroundMarker`) (`self.Selected`)))

(event `self.SetDecalHoverToAttack`
  (`DecalComponent.SetDecalMaterial` (`self.GroundMarker`) (`self.HoverMouseToAttack`)))

(event `self.SetDecalHoverToSelect`
  (`DecalComponent.SetDecalMaterial` (`self.GroundMarker`) (`self.HoverMouseToSelect`)))